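; BP_MenuPlayer is a menu character in ElfArden that displays the default weapon of a given job class.
; ShowJob looks up the job's default weapon, attaches the Weapon mesh to its socket on Body, falling back to "weapon" if none is set, then applies its mesh and grip transform.
; The Shield shows only for Warrior weapons, and both items hide when no valid weapon exists.
; The event graph and construction script are empty.
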(event EventBeginPlay)

(event Collision|EventActorBeginOverlap
  (params (OtherActor :type Actor%20Object%20Reference)))

(event EventTick
  (params (DeltaSeconds :type Float%20%28single-precision%29)))

(fn ConstructionScript)

(fn ShowJob
  (params (JobClass :type Job%20Component%20Class%20Reference))
  (bind _returnvalue (Class|JobUILibrary|GetJobDefaultWeapon JobClass))
  (bind _socketname (Variables|/Script/ZombieHunter1.WeaponDataAsset|GetSocketName _returnvalue))
  (Utilities|IsValid _returnvalue
    (:Is%20Valid
      (Transformation|AttachComponentToComponent (Variables|Default|GetWeapon) (Variables|Default|GetBody) (Utilities|String|SelectName "weapon" _socketname (== _socketname "None")) "SnapToTarget" "SnapToTarget" "KeepRelative" false)
      (Components|SkeletalMesh|SetSkeletalMeshAsset (Variables|Default|GetWeapon) (Variables|/Script/ZombieHunter1.WeaponDataAsset|GetMesh _returnvalue))
      (Transformation|SetRelativeLocationAndRotation (Variables|Default|GetWeapon) (Variables|/Script/ZombieHunter1.WeaponDataAsset|GetGripLocation _returnvalue) (Variables|/Script/ZombieHunter1.WeaponDataAsset|GetGripRotation _returnvalue) false false)
      (Rendering|SetVisibility (Variables|Default|GetWeapon) true false)
      (Rendering|SetVisibility (Variables|Default|GetShield) (Utilities|Enum|Equal(Enum) (Variables|/Script/ZombieHunter1.WeaponDataAsset|GetJobType _returnvalue) "Warrior") false))
    (:Is%20Not%20Valid
      (Rendering|SetVisibility (Variables|Default|GetWeapon) false false)
      (Rendering|SetVisibility (Variables|Default|GetShield) false false))))